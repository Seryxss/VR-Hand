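; GM_Gemmod, apparently a game mode, randomly thins the pre-placed BP_Nyamuk actors down to the InMap count when play begins.
; BeginPlay gathers every BP_Nyamuk, shuffles the array and destroys the surplus from the front, so the surviving placements vary between runs.
; Each removal decrements Total and copies it to Sisa as the remaining count.
; Tick and the construction script do nothing.
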(event `self.ReceiveBeginPlay`
  (bind _outactors (`GameplayStatics.GetAllActorsOfClass` "/Game/SpawnerNyamuk/BP_Nyamuk.BP_Nyamuk_C"))
  (`KismetArrayLibrary.Array_Shuffle` _outactors)
  (bind _returnvalue (`KismetArrayLibrary.Array_Length` _outactors))
  (set `self.Total` _returnvalue)
  (for _index (range (+ (- _returnvalue (+ (`self.InMap`) 1)) 1))
    (`self.K2_DestroyActor` (`|GetArrayItem` _outactors _index))
    (bind _output_get (set `self.Total` (- (`self.Total`) 1)))
    (set `self.Sisa` _output_get)))

(fn `UserConstructionScript`)