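; Test actor for a mosquito that flies around the player through successive points on a sphere centered on the pawn.
; Each Tick, Pathfinding lerps toward TargetPosition; on arrival, SetTargetPosition converts stepped, clamped angles and radius into the next point and a distance-based alpha increment.
; After a few points and a short delay, it re-rolls horizontal and vertical steps, steering back from pitch limits.
; Radius-step randomization is unconnected.
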(event `self.ReceiveBeginPlay`
  (`self.SetTargetPosition` 0.0 0.0 100.0)
  (set `self.CurrentXYAngle` 0.0)
  (set `self.CurrentYZAngle` 0.0)
  (set `self.CurrentRadius` 0.0))

(event `self.ReceiveTick`
  (params (DeltaSeconds :type "Float (single-precision)"))
  (`self.Pathfinding`))

(event `Pathfinding`
  (bind _returnvalue (`KismetMathLibrary.RandomFloatInRange` 2.0 10.0))
  (bind _returnvalue_2 (`KismetMathLibrary.RandomFloatInRange` 15.0 45.0))
  (bind _returnvalue_3 (+ (`self.CurrentXYAngle`) (`self.CurrentXYAngleStep`)))
  (bind _returnvalue_4 (`KismetMathLibrary.FClamp` (+ (`self.CurrentYZAngle`) (`self.CurrentYZAngleStep`)) -45.0 45.0))
  (bind _returnvalue_5 (`KismetMathLibrary.FClamp` (+ (`self.CurrentRadius`) (`self.CurrentRadiusStep`)) 100.0 300.0))
  ;[1 1 1] Cari titik baru
  (if (<= (`KismetMathLibrary.Vector_Distance` (`SceneComponent.K2_GetComponentLocation` (`self.DefaultSceneRoot`)) (`self.TargetPosition`)) 10.0)
    (set `self.HasReachedPlayer` true)
    (if (<= (- (`self.ChangeAngleAmount`) 1.0) 0.0)
      (`KismetSystemLibrary.Delay` 0.4)
      (set `self.ChangeAngleAmount` (`KismetMathLibrary.RandomIntegerInRange` 2 5))
      ;;[1 1 1] Berjalan satu arah mengelilingi sumbu Z
      (if (`KismetMathLibrary.RandomBool`)
        (set `self.CurrentXYAngleStep` (* _returnvalue_2 1.0))
        (else
          (set `self.CurrentXYAngleStep` (* _returnvalue_2 -1.0))))
      ;;[1 1 1] Berjalan satu arah mengelilingi sumbu X, limit di -45 derajat < x < 45 derajat
      (if (>= (`self.CurrentYZAngle`) 40.0)
        (set `self.CurrentYZAngleStep` (* _returnvalue -1.0) :!label _label)
        (else
          (if (<= (`self.CurrentYZAngle`) -40.0)
            _
            (elif (`KismetMathLibrary.RandomBool`)
              _
              (else
                (goto _label))))
          (set `self.CurrentYZAngleStep` (* _returnvalue 1.0))))
      ;;[1 1 1] Berjalan satu arah dalam radius
      (if (>= (`self.CurrentRadius`) 280.0)
        _
        (elif (<= (`self.CurrentRadius`) 120.0)
          _))
      (else
        ;;[1 1 1] Set Titik Baru
        (`self.SetTargetPosition` _returnvalue_3 _returnvalue_4 _returnvalue_5)
        (set `self.CurrentXYAngle` _returnvalue_3)
        (set `self.CurrentYZAngle` _returnvalue_4)
        (set `self.CurrentRadius` _returnvalue_5)
        (`/Engine/EditorBlueprintResources/StandardMacros.DecrementInt` (`self.ChangeAngleAmount`)
          (:`  `
            ;[1 1 1] Move ke target position pakai lerp
            (`self.K2_SetActorLocation` (`KismetMathLibrary.VLerp` (`SceneComponent.K2_GetComponentLocation` (`self.DefaultSceneRoot`)) (`self.TargetPosition`) (`KismetMathLibrary.FMin` (`self.CurrentLerpAlpha`) 1.0)) :!label _label_2)
            (set `self.CurrentLerpAlpha` (+ (`self.CurrentLerpAlpha`) (`self.CurrentLerpAlphaIncrement`)))))))
    (else
      (goto _label_2))))

(fn `SetTargetPosition`
  (params (xyAngle :type "Float (double-precision)") (yzAngle :type "Float (double-precision)") (radiusFromPlayer :type "Float (double-precision)"))
  (bind (_returnvalue_x _returnvalue_y _returnvalue_z) (`KismetMathLibrary.BreakVector` (`self.K2_GetActorLocation` (`GameplayStatics.GetPlayerPawn` 0))))
  (bind _returnvalue (`KismetMathLibrary.FMax` (`KismetMathLibrary.FMin` yzAngle 45.0) -45.0))
  (bind _returnvalue_2 (* (`KismetMathLibrary.DegCos` _returnvalue) radiusFromPlayer))
  (bind _output_get (set `self.TargetPosition` (`KismetMathLibrary.MakeVector` (+ _returnvalue_x (* _returnvalue_2 (`KismetMathLibrary.DegCos` xyAngle))) (+ _returnvalue_y (* _returnvalue_2 (`KismetMathLibrary.DegSin` xyAngle))) (+ _returnvalue_z (* (`KismetMathLibrary.DegSin` _returnvalue) radiusFromPlayer)))))
  (set `self.CurrentLerpAlphaIncrement` (`KismetMathLibrary.SafeDivide` 1.0 (`KismetMathLibrary.SafeDivide` (`KismetMathLibrary.Vector_Distance` (`SceneComponent.K2_GetComponentLocation` (`self.DefaultSceneRoot`)) _output_get) (`self.MoveSpeed`))))
  (set `self.CurrentLerpAlpha` 0.0))

(fn `UserConstructionScript`)