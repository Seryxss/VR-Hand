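; BP_NyamukGesit is an agile mosquito that flies around the VR player and is meant to dodge their hands.
; Pathfinding picks random, bounded angle and radius steps in runs, pausing between runs, and lerps toward each target.
; AvoidHand re-runs itself after a delay and, on proximity, cancels the pause and picks an evasive step using "Gesit" minimums.
; Both hand checks currently measure distance to the world origin, not the hands.
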(event `self.ReceiveBeginPlay`
  (`parent.ReceiveBeginPlay`)
  (bind _asbp_vrpawn (cast `/Game/Blueprint/BP_VRPawn` (`GameplayStatics.GetPlayerPawn` 0)))
  (set `self.Player` _asbp_vrpawn)
  (`self.AvoidHand`))

(event `self.Pathfinding`
  (bind _returnvalue (`KismetMathLibrary.RandomFloatInRange` (`self.MinimumXYAngleStepAmount`) (`self.MaximumXYAngleStepAmount`)))
  (bind _returnvalue_2 (`KismetMathLibrary.RandomFloatInRange` (`self.MinimumYZAngleStepAmount`) (`self.MaximumYZAngleStepAmount`)))
  (bind _returnvalue_3 (`KismetMathLibrary.RandomFloatInRange` (`self.MinimumRadiusStepAmount`) (`self.MaximumRadiusStepAmount`)))
  (bind _returnvalue_4 (+ (`self.CurrentXYAngle`) (`self.CurrentXYAngleStep`)))
  (bind _returnvalue_5 (`KismetMathLibrary.FClamp` (+ (`self.CurrentYZAngle`) (`self.CurrentYZAngleStep`)) (`self.MinimumCurrentYZAngle`) (`self.MaximumCurrentYZAngle`)))
  (bind _returnvalue_6 (`KismetMathLibrary.FClamp` (+ (`self.CurrentRadius`) (`self.CurrentRadiusStep`)) (`self.MinimumCurrentRadius`) (`self.MaximumCurrentRadius`)))
  ;[1 1 1] Cari titik baru
  (if (<= (`KismetMathLibrary.Vector_Distance` (`self.K2_GetActorLocation`) (`self.TargetPosition`)) 10.0)
    (set `self.HasReachedPlayer` true)
    (if (<= (- (`self.CurrentStepAmount`) 1.0) 0.0)
      (`KismetSystemLibrary.Delay` (`self.DelayBetweenMovement`))
      (if (`self.CancelDelay`)
        (set `self.CancelDelay` false)
        (else
          (set `self.CurrentStepAmount` (`KismetMathLibrary.RandomIntegerInRange` (`self.MinimumStepAmount`) (`self.MaximumStepAmount`)))
          ;;[1 1 1] Berjalan satu arah mengelilingi sumbu Z
          (if (`KismetMathLibrary.RandomBool`)
            (set `self.CurrentXYAngleStep` (* _returnvalue 1.0))
            (else
              (set `self.CurrentXYAngleStep` (* _returnvalue -1.0))))
          ;;[1 1 1] Berjalan satu arah mengelilingi sumbu X, limit di -45 derajat < x < 45 derajat
          (if (>= (`self.CurrentYZAngle`) (- (`self.MaximumCurrentYZAngle`) (`self.FixedYZAngleMovementThreshold`)))
            (set `self.CurrentYZAngleStep` (* _returnvalue_2 -1.0) :!label _label)
            (else
              (if (<= (`self.CurrentYZAngle`) (+ (`self.MinimumCurrentYZAngle`) (`self.FixedYZAngleMovementThreshold`)))
                _
                (elif (`KismetMathLibrary.RandomBool`)
                  _
                  (else
                    (goto _label))))
              (set `self.CurrentYZAngleStep` (* _returnvalue_2 1.0))))
          ;;[1 1 1] Berjalan satu arah dalam radius
          (if (>= (`self.CurrentRadius`) (- (`self.MaximumCurrentRadius`) (`self.FixedRadiusMovementThreshold`)))
            (set `self.CurrentRadiusStep` (* _returnvalue_3 -1.0) :!label _label_2)
            (else
              (if (<= (`self.CurrentRadius`) (+ (`self.MinimumCurrentRadius`) (`self.FixedRadiusMovementThreshold`)))
                _
                (elif (`KismetMathLibrary.RandomBool`)
                  _
                  (else
                    (goto _label_2))))
              (set `self.CurrentRadiusStep` (* _returnvalue_3 1.0))))
          ;;[1 1 1] Set Titik Baru
          (`self.SetTargetPosition` _returnvalue_4 _returnvalue_5 _returnvalue_6 :!label _label_3)
          (set `self.CurrentXYAngle` _returnvalue_4)
          (set `self.CurrentYZAngle` _returnvalue_5)
          (set `self.CurrentRadius` _returnvalue_6)
          (`/Engine/EditorBlueprintResources/StandardMacros.DecrementInt` (`self.CurrentStepAmount`)
            (:`  `
              ;[1 1 1] Move ke target position pakai lerp
              (`self.K2_SetActorLocation` (`KismetMathLibrary.VLerp` (`self.K2_GetActorLocation`) (`self.TargetPosition`) (`KismetMathLibrary.FMin` (`self.CurrentLerpAlpha`) 1.0)) :!label _label_4)
              (set `self.CurrentLerpAlpha` (+ (`self.CurrentLerpAlpha`) (`self.CurrentLerpAlphaIncrement`)))))))
      (else
        (goto _label_3)))
    (else
      (goto _label_4))))

(event `AvoidHand`
  (bind _returnvalue (`KismetMathLibrary.RandomFloatInRange` (`self.MinimumRadiusStepAmountGesit`) (`self.MaximumRadiusStepAmount`)))
  (bind _returnvalue_2 (`KismetMathLibrary.RandomFloatInRange` (`self.MinimumYZAngleStepAmoundGesit`) (`self.MaximumYZAngleStepAmount`)))
  (bind _returnvalue_3 (`KismetMathLibrary.RandomFloatInRange` (`self.MinimumXYAngleStepAmountGesit`) (`self.MaximumXYAngleStepAmount`)))
  (bind _returnvalue_4 (+ (`self.CurrentXYAngle`) (`self.CurrentXYAngleStep`)))
  (bind _returnvalue_5 (`KismetMathLibrary.FClamp` (+ (`self.CurrentYZAngle`) (`self.CurrentYZAngleStep`)) (`self.MinimumCurrentYZAngle`) (`self.MaximumCurrentYZAngle`)))
  (bind _returnvalue_6 (`KismetMathLibrary.FClamp` (+ (`self.CurrentRadius`) (`self.CurrentRadiusStep`)) (`self.MinimumCurrentRadius`) (`self.MaximumCurrentRadius`)))
  (if (<= (`KismetMathLibrary.Vector_Distance` (0.0 0.0 0.0) (`self.K2_GetActorLocation`)) (`self.AvoidThreshold`))
    ;[1 1 1] Ubah Gerakan
    ;;[1 1 1] Ubah current step dan CancelDelay
    (set `self.CurrentStepAmount` (`self.AvoidStepAmount`) :!label _label_5)
    (set `self.CancelDelay` true)
    ;;[1 1 1] Berjalan satu arah mengelilingi sumbu Z
    (if (`KismetMathLibrary.RandomBool`)
      (set `self.CurrentXYAngleStep` (* _returnvalue_3 1.0))
      (else
        (set `self.CurrentXYAngleStep` (* _returnvalue_3 -1.0))))
    ;;[1 1 1] Berjalan satu arah mengelilingi sumbu X, limit di -45 derajat < x < 45 derajat
    (if (>= (`self.CurrentYZAngle`) (- (`self.MaximumCurrentYZAngle`) (`self.FixedYZAngleMovementThreshold`)))
      (set `self.CurrentYZAngleStep` (* _returnvalue_2 -1.0) :!label _label_6)
      (else
        (if (<= (`self.CurrentYZAngle`) (+ (`self.MinimumCurrentYZAngle`) (`self.FixedYZAngleMovementThreshold`)))
          _
          (elif (`KismetMathLibrary.RandomBool`)
            _
            (else
              (goto _label_6))))
        (set `self.CurrentYZAngleStep` (* _returnvalue_2 1.0))))
    ;;[1 1 1] Berjalan satu arah dalam radius
    (if (>= (`self.CurrentRadius`) (- (`self.MaximumCurrentRadius`) (`self.FixedRadiusMovementThreshold`)))
      (set `self.CurrentRadiusStep` (* _returnvalue -1.0) :!label _label_7)
      (else
        (if (<= (`self.CurrentRadius`) (+ (`self.MinimumCurrentRadius`) (`self.FixedRadiusMovementThreshold`)))
          _
          (elif (`KismetMathLibrary.RandomBool`)
            _
            (else
              (goto _label_7))))
        (set `self.CurrentRadiusStep` (* _returnvalue 1.0))))
    ;;[1 1 1] Set Titik Baru
    (`self.SetTargetPosition` _returnvalue_4 _returnvalue_5 _returnvalue_6)
    (set `self.CurrentXYAngle` _returnvalue_4)
    (set `self.CurrentYZAngle` _returnvalue_5)
    (set `self.CurrentRadius` _returnvalue_6)
    (`/Engine/EditorBlueprintResources/StandardMacros.DecrementInt` (`self.CurrentStepAmount`)
      (:`  `
        _))
    (elif (<= (`KismetMathLibrary.Vector_Distance` (0.0 0.0 0.0) (`self.K2_GetActorLocation`)) (`self.AvoidThreshold`))
      (goto _label_5)
      (else
        _)))
  ;[1 1 1] Recursive Call
  (`KismetSystemLibrary.Delay` (`self.AvoidHandDelay`))
  (`self.AvoidHand`))

(fn `UserConstructionScript`
  (`parent.UserConstructionScript`))