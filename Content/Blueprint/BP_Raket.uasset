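; BP_Raket is a VR electric racket that destroys BP_Nyamuk (mosquito) actors on contact.
; When the pawn overlaps the handle, it calls Grab and, if pinching, attaches the racket mesh to that hand's palm socket.
; Pickup enables shocking and updates the pawn's held-racket state, with no release logic here.
; Four box overlaps share one destroy call targeting all four cast results, gated by CanShock.
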(event `self.Handle.OnComponentBeginOverlap`
  (params (OverlappedComponent :type "PrimitiveComponent Object Reference") (OtherActor :type "Actor Object Reference") (OtherComp :type "PrimitiveComponent Object Reference") (OtherBodyIndex :type Integer) (bFromSweep :type Boolean) (SweepResult :type "HitResult Structure (by ref)"))
  (bind _electricracket_sketchfab (`self.ElectricRacket_sketchfab`))
  (if (not (`self.PickedUp`))
    (bind _asbp_vrpawn (cast `/Game/Blueprint/BP_VRPawn` OtherActor))
    (`/Game/Blueprint/BP_VRPawn.Grab` _asbp_vrpawn)
    (bind _pinchright (`/Game/Blueprint/BP_VRPawn.PinchRight` _asbp_vrpawn))
    (if (or _pinchright (`/Game/Blueprint/BP_VRPawn.PinchLeft` _asbp_vrpawn))
      (if _pinchright
        (`SceneComponent.K2_AttachToComponent` _electricracket_sketchfab (`/Game/Blueprint/BP_VRPawn.OculusXRHandR` _asbp_vrpawn) "r_palm_center_marker" "KeepWorld" "KeepWorld" "KeepWorld" true)
        (else
          (`SceneComponent.K2_AttachToComponent` _electricracket_sketchfab (`/Game/Blueprint/BP_VRPawn.OculusXRHandL` _asbp_vrpawn) "l_palm_center_marker" "KeepWorld" "KeepWorld" "KeepWorld" true)))
      (set `self.CanShock` true)
      (set `self.PickedUp` true)
      (set `/Game/Blueprint/BP_VRPawn.Hand` false _asbp_vrpawn)
      (set `/Game/Blueprint/BP_VRPawn.Racket` true _asbp_vrpawn)
      (set `/Game/Blueprint/BP_VRPawn.RacketHeld` self _asbp_vrpawn))))

(event `self.Box.OnComponentBeginOverlap`
  (params (OverlappedComponent :type "PrimitiveComponent Object Reference") (OtherActor :type "Actor Object Reference") (OtherComp :type "PrimitiveComponent Object Reference") (OtherBodyIndex :type Integer) (bFromSweep :type Boolean) (SweepResult :type "HitResult Structure (by ref)"))
  (bind _asbp_nyamuk (cast `/Game/Blueprint/BP_Nyamuk` OtherActor))
  (if (`self.CanShock`) :!label _label
    (`self.K2_DestroyActor` _asbp_nyamuk)
    (`self.K2_DestroyActor` (stale `self.Box3.OnComponentBeginOverlap` _asbp_nyamuk))
    (`self.K2_DestroyActor` (stale `self.Box2.OnComponentBeginOverlap` _asbp_nyamuk))
    (`self.K2_DestroyActor` (stale `self.Box1.OnComponentBeginOverlap` _asbp_nyamuk))))

(event `self.Box1.OnComponentBeginOverlap`
  (params (OverlappedComponent :type "PrimitiveComponent Object Reference") (OtherActor :type "Actor Object Reference") (OtherComp :type "PrimitiveComponent Object Reference") (OtherBodyIndex :type Integer) (bFromSweep :type Boolean) (SweepResult :type "HitResult Structure (by ref)"))
  (bind _asbp_nyamuk (cast `/Game/Blueprint/BP_Nyamuk` OtherActor))
  (goto _label))

(event `self.Box2.OnComponentBeginOverlap`
  (params (OverlappedComponent :type "PrimitiveComponent Object Reference") (OtherActor :type "Actor Object Reference") (OtherComp :type "PrimitiveComponent Object Reference") (OtherBodyIndex :type Integer) (bFromSweep :type Boolean) (SweepResult :type "HitResult Structure (by ref)"))
  (bind _asbp_nyamuk (cast `/Game/Blueprint/BP_Nyamuk` OtherActor))
  (goto _label))

(event `self.Box3.OnComponentBeginOverlap`
  (params (OverlappedComponent :type "PrimitiveComponent Object Reference") (OtherActor :type "Actor Object Reference") (OtherComp :type "PrimitiveComponent Object Reference") (OtherBodyIndex :type Integer) (bFromSweep :type Boolean) (SweepResult :type "HitResult Structure (by ref)"))
  (bind _asbp_nyamuk (cast `/Game/Blueprint/BP_Nyamuk` OtherActor))
  (goto _label))

(fn `UserConstructionScript`)