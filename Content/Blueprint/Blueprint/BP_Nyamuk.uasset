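; BP_Nyamuk is a VR mosquito that hovers around the player until a hand kills it.
; Each tick it lerps toward a target in spherical coordinates around the player, with clamped elevation and radius.
; On arrival it steps onward, periodically pausing to randomize step count and directions, steering away from limits.
; An overlap kills it with a Niagara burst if the pawn's HandCollide and CanKill are true; physical hits retarget it and zero velocity.
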(event `self.ReceiveBeginPlay`
  (`self.SetTargetPosition` 0.0 0.0 100.0)
  (set `self.CurrentXYAngle` 0.0)
  (set `self.CurrentYZAngle` 0.0)
  (set `self.CurrentRadius` 0.0))

(event `self.ReceiveTick`
  (params (DeltaSeconds :type "Float (single-precision)"))
  (`self.Pathfinding`))

(event `self.Collide.OnComponentBeginOverlap`
  (params (OverlappedComponent :type "PrimitiveComponent Object Reference") (OtherActor :type "Actor Object Reference") (OtherComp :type "PrimitiveComponent Object Reference") (OtherBodyIndex :type Integer) (bFromSweep :type Boolean) (SweepResult :type "HitResult Structure (by ref)"))
  (bind _asbp_vrpawn (cast `/Game/Blueprint/Blueprint/BP_VRPawn` OtherActor))
  (if (and (`/Game/Blueprint/Blueprint/BP_VRPawn.HandCollide` _asbp_vrpawn) (`/Game/Blueprint/Blueprint/BP_VRPawn.CanKill` _asbp_vrpawn))
    (`NiagaraFunctionLibrary.SpawnSystemAtLocation` "/Game/Blueprints/NS_MosquitoBurst.NS_MosquitoBurst" (`self.K2_GetActorLocation` self))
    (`self.K2_DestroyActor`)
    (set `/Game/Blueprint/Blueprint/BP_VRPawn.CanKill` false _asbp_vrpawn)))

(event `Pathfinding`
  (bind _returnvalue (`KismetMathLibrary.RandomFloatInRange` (`self.MinimumRadiusStepAmount`) (`self.MaximumRadiusStepAmount`)))
  (bind _returnvalue_2 (`KismetMathLibrary.RandomFloatInRange` (`self.MinimumYZAngleStepAmount`) (`self.MaximumYZAngleStepAmount`)))
  (bind _returnvalue_3 (`KismetMathLibrary.RandomFloatInRange` (`self.MinimumXYAngleStepAmount`) (`self.MaximumXYAngleStepAmount`)))
  (bind _returnvalue_4 (+ (`self.CurrentXYAngle`) (`self.CurrentXYAngleStep`)))
  (bind _returnvalue_5 (`KismetMathLibrary.FClamp` (+ (`self.CurrentYZAngle`) (`self.CurrentYZAngleStep`)) (`self.MinimumCurrentYZAngle`) (`self.MaximumCurrentYZAngle`)))
  (bind _returnvalue_6 (`KismetMathLibrary.FClamp` (+ (`self.CurrentRadius`) (`self.CurrentRadiusStep`)) (`self.MinimumCurrentRadius`) (`self.MaximumCurrentRadius`)))
  ;[1 1 1] Cari titik baru
  (if (<= (`KismetMathLibrary.Vector_Distance` (`self.K2_GetActorLocation`) (`self.TargetPosition`)) 10.0)
    (set `self.HasReachedPlayer` true)
    (if (<= (- (`self.CurrentStepAmount`) 1.0) 0.0)
      (`KismetSystemLibrary.Delay` (`self.DelayBetweenMovement`))
      (set `self.CurrentStepAmount` (`KismetMathLibrary.RandomIntegerInRange` (`self.MinimumStepAmount`) (`self.MaximumStepAmount`)))
      ;;[1 1 1] Berjalan satu arah mengelilingi sumbu Z
      (if (`KismetMathLibrary.RandomBool`)
        (set `self.CurrentXYAngleStep` (* _returnvalue_3 1.0))
        (else
          (set `self.CurrentXYAngleStep` (* _returnvalue_3 -1.0))))
      ;;[1 1 1] Berjalan satu arah mengelilingi sumbu X, limit di -45 derajat < x < 45 derajat
      (if (>= (`self.CurrentYZAngle`) (- (`self.MaximumCurrentYZAngle`) (`self.FixedYZAngleMovementThreshold`)))
        (set `self.CurrentYZAngleStep` (* _returnvalue_2 -1.0) :!label _label)
        (else
          (if (<= (`self.CurrentYZAngle`) (+ (`self.MinimumCurrentYZAngle`) (`self.FixedYZAngleMovementThreshold`)))
            _
            (elif (`KismetMathLibrary.RandomBool`)
              _
              (else
                (goto _label))))
          (set `self.CurrentYZAngleStep` (* _returnvalue_2 1.0))))
      ;;[1 1 1] Berjalan satu arah dalam radius
      (if (>= (`self.CurrentRadius`) (- (`self.MaximumCurrentRadius`) (`self.FixedRadiusMovementThreshold`)))
        (set `self.CurrentRadiusStep` (* _returnvalue -1.0) :!label _label_2)
        (else
          (if (<= (`self.CurrentRadius`) (+ (`self.MinimumCurrentRadius`) (`self.FixedRadiusMovementThreshold`)))
            _
            (elif (`KismetMathLibrary.RandomBool`)
              _
              (else
                (goto _label_2))))
          (set `self.CurrentRadiusStep` (* _returnvalue 1.0)))))
    ;;[1 1 1] Set Titik Baru
    (`self.SetTargetPosition` _returnvalue_4 _returnvalue_5 _returnvalue_6)
    (set `self.CurrentXYAngle` _returnvalue_4)
    (set `self.CurrentYZAngle` _returnvalue_5)
    (set `self.CurrentRadius` _returnvalue_6)
    (`/Engine/EditorBlueprintResources/StandardMacros.DecrementInt` (`self.CurrentStepAmount`)
      (:`  `
        _)))
  ;[1 1 1] Move ke target position pakai lerp
  (`self.K2_SetActorLocation` (`KismetMathLibrary.VLerp` (`self.K2_GetActorLocation`) (`self.TargetPosition`) (`KismetMathLibrary.FMin` (`self.CurrentLerpAlpha`) 1.0)))
  (set `self.CurrentLerpAlpha` (+ (`self.CurrentLerpAlpha`) (`self.CurrentLerpAlphaIncrement`))))

(event `self.Sphere.OnComponentHit`
  (params (HitComponent :type "PrimitiveComponent Object Reference") (OtherActor :type "Actor Object Reference") (OtherComp :type "PrimitiveComponent Object Reference") (NormalImpulse :type "Vector Structure") (Hit :type "HitResult Structure (by ref)"))
  (bind _sphere (`self.Sphere`))
  ;[1 1 1] Cari titik baru ketika kena tangan. Kadang masih jitter" aneh
  (cast `/Game/Blueprint/Blueprint/BP_VRPawn` OtherActor)
  (`KismetSystemLibrary.PrintString` "Nyamuk start hit hand")
  (`self.SetTargetPosition` (`self.CurrentXYAngle`) (`self.CurrentYZAngle`) (`self.CurrentRadius`))
  (`KismetSystemLibrary.PrintString` (`KismetStringLibrary.Conv_VectorToString` (`SceneComponent.GetComponentVelocity` _sphere)))
  (`PrimitiveComponent.SetAllPhysicsLinearVelocity` _sphere (0.0 0.0 0.0) false))

(fn `SetTargetPosition`
  (params (xyAngle :type "Float (double-precision)") (yzAngle :type "Float (double-precision)") (radiusFromPlayer :type "Float (double-precision)"))
  (bind (_returnvalue_x _returnvalue_y _returnvalue_z) (`KismetMathLibrary.BreakVector` (`self.K2_GetActorLocation` (`GameplayStatics.GetPlayerPawn` 0))))
  (bind _returnvalue (`KismetMathLibrary.FMax` (`KismetMathLibrary.FMin` yzAngle 45.0) -45.0))
  (bind _returnvalue_2 (* (`KismetMathLibrary.DegCos` _returnvalue) radiusFromPlayer))
  (bind _output_get (set `self.TargetPosition` (`KismetMathLibrary.MakeVector` (+ _returnvalue_x (* _returnvalue_2 (`KismetMathLibrary.DegCos` xyAngle))) (+ _returnvalue_y (* _returnvalue_2 (`KismetMathLibrary.DegSin` xyAngle))) (+ (+ _returnvalue_z (* (`KismetMathLibrary.DegSin` _returnvalue) radiusFromPlayer)) (`self.ZOffset`)))))
  (set `self.CurrentLerpAlphaIncrement` (`KismetMathLibrary.SafeDivide` 1.0 (`KismetMathLibrary.SafeDivide` (`KismetMathLibrary.Vector_Distance` (`self.K2_GetActorLocation`) _output_get) (`self.MoveSpeed`))))
  (set `self.CurrentLerpAlpha` 0.0))

(fn `UserConstructionScript`)